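; Player character with multi-jump, backflip, dash, landing camera shake and switchable TPS/skin cameras, configured from BP_GameInstance.
; Tick traces downward to save the last navmesh-projected ground point as the respawn transform.
; Exceeding the fall-velocity limit kills mid-air: it ragdolls, leaves a numbered BP_Grave there and clears BP_Cadavre actors.
; A replacement character is possessed at that point, or at PlayerStart with lives and timer reset when none remain.
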(event Custom|Dash
  (bind _returnvalue (Transformation|GetActorForwardVector))
  (Utilities|FlowControl|DoOnce false :!label _label
    (:Completed
      (if (Variables|Default|GetCanDash)
        (Variables|Default|SetCanDash false)
        (Character|LaunchCharacter (* (Transformation|GetActorUpVector) 1e+02) false true)
        (Utilities|FlowControl|Delay 0.1)
        (Character|LaunchCharacter (* (Math|Vector|Normalize (Math|Vector|MakeVector (.x _returnvalue) (.y _returnvalue) 0.0)) 1e+03) true false)
        (Animation|Montage|PlayMontage (Variables|Character|GetMesh) "/Game/LD57/Animations/AM_DashJump.AM_DashJump"
          (:OnCompleted
            (goto _label Reset)))
        (else
          (goto _label Reset))))))

(event Custom|LandedDelegate_Event
  (params (Hit :type Hit%20Result%20Structure%20%28by%20ref%29))
  (bind _charactermovement (Variables|Character|GetCharacterMovement))
  (bind _returnvalue (Pawn|Components|CharacterMovement|GetLastUpdateVelocity _charactermovement))
  (if (< (.z _returnvalue) 0.0)
    (if (Variables|/Game/LD57/Blueprints/BP_GameInstance.BP_GameInstance_C|GetEnableShake (Variables|Default|GetGameInstance))
      (Game|Feedback|ClientStartCameraShake (Game|GetPlayerController 0) "/Game/LD57/Blueprints/Player/BP_DamageCameraShake.BP_DamageCameraShake_C" (/ (.z _returnvalue) (Default|GetVelocityMax (Variables|Default|GetGameInstance))) "CameraLocal" "0, 0, 0")))
  (Variables|Default|SetCanDash true)
  (Variables|Default|SetHasDoneFirstJump false))

(event Custom|DoJump
  (if (Character|CanJump)
    (if (Variables|Default|GetHasDoneFirstJump)
      (Audio|PlaySoundatLocation "/Game/LD57/Sound/Sc_DoubleJump.Sc_DoubleJump" (Transformation|GetActorLocation) "0, 0, 0" 1.0 1.0 0.0 0 0 0 0)
      (Animation|Montage|PlayMontage (Variables|Character|GetMesh) "/Game/LD57/Animations/AM_Backflip.AM_Backflip" 1.5 0.3
        (:then
          _)))
    (Character|Jump)
    (Variables|Default|SetHasDoneFirstJump true)))

(event EventBeginPlay
  (bind _asbp_game_instance (Utilities|Casting|CastToBP_GameInstance (Game|GetGameInstance)))
  (bind _output_get (Variables|Default|SetGameInstance _asbp_game_instance))
  (Variables|Default|SetJumpMaxCount (Default|GetMaxJumpCount _output_get))
  (Variables|/Script/Engine.CharacterMovementComponent|SetAirControl (Variables|Character|GetCharacterMovement) (Default|GetAirControlValue (Variables|Default|GetGameInstance)))
  (EventDispatchers|BindEventtoLandedDelegate (delegate Custom|LandedDelegate_Event))
  (Components|SkeletalMesh|SetSkeletalMeshAsset (Variables|Character|GetMesh) (Variables|/Game/LD57/Blueprints/BP_GameInstance.BP_GameInstance_C|GetSelectedSkin (Variables|Default|GetGameInstance)))
  (Variables|Default|SetCanDash true)
  (Variables|Default|SetHasDoneFirstJump false))

(event EventTick
  (params (DeltaSeconds :type Float%20%28single-precision%29))
  (bind _returnvalue (Game|GetPlayerController 0))
  (bind _returnvalue_2 (Transformation|GetActorLocation))
  (bind _gameinstance (Variables|Default|GetGameInstance))
  (bind _gameinstance_2 (Variables|Default|GetGameInstance))
  (bind _gameinstance_3 (Variables|Default|GetGameInstance))
  (bind _gameinstance_4 (Variables|Default|GetGameInstance))
  (Utilities|FlowControl|Sequence
    (:then_0
      (if (not (Variables|Default|GetIsDead))
        (bind (_outhit _returnvalue_3) (Collision|SphereTraceByChannel _returnvalue_2 (- _returnvalue_2 "0.000000,0.000000,100.000000") 2e+01 "TraceTypeQuery1" false 0 "None"))
        (if _returnvalue_3
          (if (.ReturnValue (AI|Navigation|ProjectPointtoNavigation (.impactpoint _outhit) 0 0 "0, 0, 0"))
            (Variables|/Game/LD57/Blueprints/BP_GameInstance.BP_GameInstance_C|SetLastTransform (Variables|Default|GetGameInstance) (Math|Transform|MakeTransform (.ProjectedLocation (AI|Navigation|ProjectPointtoNavigation (.impactpoint _outhit) 0 0 "0, 0, 0")) (Transformation|GetActorRotation) "1.000000,1.000000,1.000000"))))))
    (:then_1
      (if (and (> (Default|GetVelocityMax (Variables|Default|GetGameInstance)) (.z (Transformation|GetVelocity))) (not (Variables|Default|GetIsDead)))
        (Audio|PlaySound2D "/Game/LD57/Sound/deathSound/SC_Wilhelm.SC_Wilhelm" 1.0 1.0 0.0 0 0)
        (Physics|SetSimulatePhysics (Variables|Character|GetMesh) true)
        (Variables|Default|SetIsDead true)
        (Utilities|FlowControl|Delay 1.5)
        (Game|SpawnActorfromClass "/Game/LD57/Blueprints/BP_Grave.BP_Grave_C" (Math|Transform|MakeTransform (.location (Variables|/Game/LD57/Blueprints/BP_GameInstance.BP_GameInstance_C|GetLastTransform _gameinstance_4)) (Math|Rotator|MakeRotator 0.0 0.0 (+ (.yaw (.rotation (Variables|/Game/LD57/Blueprints/BP_GameInstance.BP_GameInstance_C|GetLastTransform _gameinstance_4))) 1.8e+02)) "1.000000,1.000000,1.000000") "AlwaysSpawn" "MultiplyWithRoot" 0 (+ (Variables|/Game/LD57/Blueprints/BP_GameInstance.BP_GameInstance_C|GetTotalLifeWasted _gameinstance_4) 1) 0)
        (Utilities|FlowControl|Sequence
          (:then_0
            (bind _outactors (Actor|GetAllActorsOfClass "/Game/LD57/Blueprints/LD/BP_Cadavre.BP_Cadavre_C"))
            (for _array_element _outactors
              (Actor|DestroyActor _array_element)))
          (:then_1
            (Variables|/Game/LD57/Blueprints/BP_GameInstance.BP_GameInstance_C|SetTotalLifeWasted _gameinstance_2 (+ (Variables|/Game/LD57/Blueprints/BP_GameInstance.BP_GameInstance_C|GetTotalLifeWasted _gameinstance_2) 1))
            (if (> (Variables|/Game/LD57/Blueprints/BP_GameInstance.BP_GameInstance_C|GetCurrentLife _gameinstance_2) 0)
              (Variables|/Game/LD57/Blueprints/BP_GameInstance.BP_GameInstance_C|SetCurrentLife _gameinstance (- (Variables|/Game/LD57/Blueprints/BP_GameInstance.BP_GameInstance_C|GetCurrentLife _gameinstance) 1))
              (bind _returnvalue_4 (Game|SpawnActorfromClass "BP_PlayerCharacter_C" (Math|Transform|MakeTransform (+ (.location (Variables|/Game/LD57/Blueprints/BP_GameInstance.BP_GameInstance_C|GetLastTransform _gameinstance)) "0.000000,0.000000,90.000000") (.rotation (Variables|/Game/LD57/Blueprints/BP_GameInstance.BP_GameInstance_C|GetLastTransform _gameinstance)) "1.000000,1.000000,1.000000") "AdjustIfPossibleButAlwaysSpawn" "MultiplyWithRoot" 0 0))
              (Pawn|UnPossess _returnvalue)
              (Pawn|Possess _returnvalue _returnvalue_4)
              (else
                (Variables|/Game/LD57/Blueprints/BP_GameInstance.BP_GameInstance_C|SetCurrentLife _gameinstance (Default|GetMaxLifeCount _gameinstance))
                (bind _returnvalue_5 (Actor|GetActorOfClass "/Script/Engine.PlayerStart"))
                (bind _returnvalue_6 (Game|SpawnActorfromClass "BP_PlayerCharacter_C" (Math|Transform|MakeTransform (+ (.location (Transformation|GetActorTransform _returnvalue_5)) "0.000000,0.000000,90.000000") (.rotation (Transformation|GetActorTransform _returnvalue_5)) "1.000000,1.000000,1.000000") "AdjustIfPossibleButAlwaysSpawn" "MultiplyWithRoot" 0 0))
                (Variables|/Game/LD57/Blueprints/BP_GameInstance.BP_GameInstance_C|SetRunTimer _gameinstance_3 false)
                (Variables|/Game/LD57/Blueprints/BP_GameInstance.BP_GameInstance_C|SetTimer _gameinstance_3 0.0)
                (Pawn|UnPossess _returnvalue)
                (Pawn|Possess _returnvalue _returnvalue_6)))
            (Actor|DestroyActor)))))))

(fn ConstructionScript
  (|CallParentFunction))

(fn SwitchCamera
  (params (TPS :type Boolean))
  (bind _skincamera (Variables|Default|GetSkinCamera))
  (bind _tpscamera (Variables|Default|GetTPSCamera))
  (Components|Activation|SetActive (Variables|Default|GetSkinCamera) false false)
  (Components|Activation|SetActive (Variables|Default|GetTPSCamera) false false)
  (if TPS
    (Components|Activation|SetActive _tpscamera true false)
    (return _tpscamera)
    (else
      (Components|Activation|SetActive _skincamera true false)
      (return _skincamera))))