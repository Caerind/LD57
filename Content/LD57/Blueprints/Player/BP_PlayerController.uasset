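; Player controller for a third-person game with clicking, money and upgrades, owning input, the HUD and menu screens.
; Enhanced Input drives movement, dash, time slow and camera-traced clicks on BPI_Clickable actors, blocked while skin, settings or username screens are open.
; Tick updates GameInstance money and run timer, refreshes HUD and crosshair, and scales camera FOV with fall speed when enabled.
; Debug keys include a money cheat.
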(event Input|EnhancedActionEvents|EnhancedInputActionIA_Move
  (params (ActionValue :type Vector%202D%20Structure) (ElapsedSeconds :type Float%20%28double-precision%29) (TriggeredSeconds :type Float%20%28double-precision%29) (InputAction :type Input%20Action%20Object%20Reference :default "/Game/LD57/Input/Actions/IA_Move.IA_Move"))
  (bind _returnvalue (Pawn|GetControlledPawn))
  (bind _returnvalue_2 (Pawn|GetControlRotation _returnvalue :!class /Script/Engine.Pawn))
  (if (Math|Boolean|ANDBoolean (not (Variables|Default|GetSkinOpen)) (Utilities|IsValid (Variables|Default|GetPlayerCharacter)) (not (Variables|Default|GetSettingsOpen)) (not (Variables|Default|GetUsernameOpen)))
    (Utilities|IsValid _returnvalue
      (:Is%20Valid
        (Pawn|Input|AddMovementInput _returnvalue (Math|Vector|GetForwardVector (Math|Rotator|MakeRotator 0.0 0.0 (.yaw (Pawn|GetControlRotation _returnvalue :!class /Script/Engine.Pawn)))) (.y ActionValue) false)
        (Pawn|Input|AddMovementInput _returnvalue (Math|Vector|GetRightVector (Math|Rotator|MakeRotator (.roll _returnvalue_2) 0.0 (.yaw _returnvalue_2))) (.x ActionValue) false)))))

(event Input|EnhancedActionEvents|EnhancedInputActionIA_Look
  (params (ActionValue :type Vector%202D%20Structure) (ElapsedSeconds :type Float%20%28double-precision%29) (TriggeredSeconds :type Float%20%28double-precision%29) (InputAction :type Input%20Action%20Object%20Reference :default "/Game/LD57/Input/Actions/IA_Look.IA_Look"))
  (bind _returnvalue (Pawn|GetControlledPawn))
  (if (Math|Boolean|ANDBoolean (not (Variables|Default|GetSkinOpen)) (Utilities|IsValid (Variables|Default|GetPlayerCharacter)) (not (Variables|Default|GetSettingsOpen)) (not (Variables|Default|GetUsernameOpen)))
    (Pawn|Input|AddControllerYawInput _returnvalue (.x ActionValue))
    (Pawn|Input|AddControllerPitchInput _returnvalue (* (.y ActionValue) (Math|Float|SelectFloat -1.0 1.0 false)))))

(event Input|EnhancedActionEvents|EnhancedInputActionIA_Jump
  (params (ActionValue :type Boolean) (ElapsedSeconds :type Float%20%28double-precision%29) (TriggeredSeconds :type Float%20%28double-precision%29) (InputAction :type Input%20Action%20Object%20Reference :default "/Game/LD57/Input/Actions/IA_Jump.IA_Jump"))
  (bind _playercharacter (Variables|Default|GetPlayerCharacter))
  (:Started
    (if (Math|Boolean|ANDBoolean (not (Variables|Default|GetSkinOpen)) (Utilities|IsValid (Variables|Default|GetPlayerCharacter)) (not (Variables|Default|GetSettingsOpen)) (not (Variables|Default|GetUsernameOpen)))
      (Default|DoJump _playercharacter)))
  (:Completed
    (if (Math|Boolean|ANDBoolean (not (Variables|Default|GetSkinOpen)) (Utilities|IsValid (Variables|Default|GetPlayerCharacter)) (not (Variables|Default|GetSettingsOpen)) (not (Variables|Default|GetUsernameOpen)))
      (Character|StopJumping _playercharacter))))

(event Input|EnhancedActionEvents|EnhancedInputActionIA_Click
  (params (ActionValue :type Boolean) (ElapsedSeconds :type Float%20%28double-precision%29) (TriggeredSeconds :type Float%20%28double-precision%29) (InputAction :type Input%20Action%20Object%20Reference :default "/Game/LD57/Input/Actions/IA_Click.IA_Click"))
  (:Started
    (if (Math|Boolean|ANDBoolean (not (Variables|Default|GetSkinOpen)) (Utilities|IsValid (Variables|Default|GetPlayerCharacter)) (not (Variables|Default|GetSettingsOpen)) (not (Variables|Default|GetUsernameOpen)))
      (bind (_clicklocation _valid _clickable _actor) (CallFunction|GetClickLocation))
      (if _valid
        (if _clickable
          (bind _result (Class|BPIClickable|OnClick(Message) _actor _clicklocation))
          (if _result
            (Niagara|SpawnSystematLocation "/Game/LD57/FX/NS_ElecGreen.NS_ElecGreen" _clicklocation "0, 0, 0" "1.500000,1.500000,1.500000")
            (else
              (Niagara|SpawnSystematLocation "/Game/LD57/FX/NS_ElecBlue.NS_ElecBlue" _clicklocation "0, 0, 0" "1.500000,1.500000,1.500000"))))))))

(event Input|EnhancedActionEvents|EnhancedInputActionIA_TimeSlow
  (params (ActionValue :type Boolean) (ElapsedSeconds :type Float%20%28double-precision%29) (TriggeredSeconds :type Float%20%28double-precision%29) (InputAction :type Input%20Action%20Object%20Reference :default "/Game/LD57/Input/Actions/IA_TimeSlow.IA_TimeSlow"))
  (bind _gameinstance (Variables|Default|GetGameInstance))
  (:Started
    (if (Math|Boolean|ANDBoolean (not (Variables|Default|GetSkinOpen)) (Utilities|IsValid (Variables|Default|GetPlayerCharacter)) (not (Variables|Default|GetSettingsOpen)) (not (Variables|Default|GetUsernameOpen)))
      (if (Default|CanUseSkill _gameinstance "NewEnumerator0")
        (Utilities|Time|SetGlobalTimeDilation (Default|GetTimeSlowFactor _gameinstance))
        (Utilities|FlowControl|Delay (Default|GetTimeSlowDuration _gameinstance))
        (Utilities|Time|SetGlobalTimeDilation 1.0)))))

(event Input|EnhancedActionEvents|EnhancedInputActionIA_Dash
  (params (ActionValue :type Boolean) (ElapsedSeconds :type Float%20%28double-precision%29) (TriggeredSeconds :type Float%20%28double-precision%29) (InputAction :type Input%20Action%20Object%20Reference :default "/Game/LD57/Input/Actions/IA_Dash.IA_Dash"))
  (:Started
    (if (Math|Boolean|ANDBoolean (not (Variables|Default|GetSkinOpen)) (Utilities|IsValid (Variables|Default|GetPlayerCharacter)) (not (Variables|Default|GetSettingsOpen)) (not (Variables|Default|GetUsernameOpen)))
      (if (Default|CanUseSkill (Variables|Default|GetGameInstance) "NewEnumerator5")
        (Default|Dash (Variables|Default|GetPlayerCharacter))))))

(event Input|EnhancedActionEvents|EnhancedInputActionIA_Skin
  (params (ActionValue :type Boolean) (ElapsedSeconds :type Float%20%28double-precision%29) (TriggeredSeconds :type Float%20%28double-precision%29) (InputAction :type Input%20Action%20Object%20Reference :default "/Game/LD57/Input/Actions/IA_Skin.IA_Skin"))
  (:Started
    (if (.unlocked (Default|GetUpgrade (Variables|Default|GetGameInstance) "NewEnumerator13"))
      (CallFunction|ToggleSkin))))

(event Input|EnhancedActionEvents|EnhancedInputActionIA_Setttings
  (params (ActionValue :type Boolean) (ElapsedSeconds :type Float%20%28double-precision%29) (TriggeredSeconds :type Float%20%28double-precision%29) (InputAction :type Input%20Action%20Object%20Reference :default "/Game/LD57/Input/Actions/IA_Setttings.IA_Setttings"))
  (:Started
    (if (not (Variables|Default|GetUsernameOpen))
      (CallFunction|ToggleSettings))))

(event EventBeginPlay
  (bind _asbp_game_mode (Utilities|Casting|CastToBP_GameMode (Game|GetGameMode)))
  (Variables|Default|SetGameMode _asbp_game_mode)
  (bind _asbp_game_instance (Utilities|Casting|CastToBP_GameInstance (Game|GetGameInstance)))
  (Variables|Default|SetGameInstance _asbp_game_instance)
  (Audio|PlaySound2D "/Game/LD57/Sound/Ambiance/SD_Ambiance.SD_Ambiance" 1.0 1.0 0.0 0 0)
  (Input|AddMappingContext (PlayerController|LocalPlayerSubsystems|GetEnhancedInputLocalPlayerSubsystem) "/Game/LD57/Input/IMC_Default.IMC_Default" 0 "(bIgnoreAllPressedKeysUntilRelease=True,bForceImmediately=False,bNotifyUserSettings=False)")
  (bind _returnvalue (Game|ConstructObjectfromClass "/Game/LD57/Blueprints/UI/WBP_HUD.WBP_HUD_C"))
  (bind _output_get (Variables|Default|SetHUD _returnvalue))
  (Variables|/Game/LD57/Blueprints/BP_GameInstance.BP_GameInstance_C|SetHUD (Variables|Default|GetGameInstance) _output_get)
  (bind _returnvalue_2 (Game|ConstructObjectfromClass "/Game/LD57/Blueprints/UI/WBP_Skins.WBP_Skins_C"))
  (Variables|Default|SetSkinScreen _returnvalue_2)
  (bind _returnvalue_3 (Game|ConstructObjectfromClass "/Game/LD57/Blueprints/UI/WBP_Settings.WBP_Settings_C"))
  (Variables|Default|SetSettingsScreen _returnvalue_3)
  (if (== (Utilities|String|Len (Variables|/Game/LD57/Blueprints/BP_GameInstance.BP_GameInstance_C|GetUsername (Variables|Default|GetGameInstance))) 0)
    (bind _returnvalue_4 (Game|ConstructObjectfromClass "/Game/LD57/Blueprints/UI/WBP_Username.WBP_Username_C"))
    (bind _output_get_2 (Variables|Default|SetUsernameScreen _returnvalue_4))
    (UserInterface|Viewport|AddtoViewport _output_get_2 0)
    (Variables|Default|SetbShowMouseCursor true)
    (Variables|Default|SetUsernameOpen true)))

(event EventTick
  (params (DeltaSeconds :type Float%20%28single-precision%29))
  (bind _gameinstance (Variables|Default|GetGameInstance))
  (bind _gameinstance_2 (Variables|Default|GetGameInstance))
  (Utilities|IsValid (Variables|Default|GetPlayerCharacter)
    (:Is%20Valid
      (Utilities|FlowControl|Sequence
        (:then_0
          (Utilities|IsValid (Variables|Default|GetUsernameScreen)
            (:Is%20Valid
              (if (> (Utilities|String|Len (Variables|/Game/LD57/Blueprints/BP_GameInstance.BP_GameInstance_C|GetUsername (Variables|Default|GetGameInstance))) 0)
                (Widget|RemovefromParent (Variables|Default|GetUsernameScreen))
                (Variables|Default|SetUsernameScreen 0)
                (Variables|Default|SetbShowMouseCursor false)
                (Variables|Default|SetUsernameOpen false)
                (UserInterface|Viewport|AddtoViewport (Variables|Default|GetHUD) 0)
                (Variables|Default|SetHUDOpen true)))))
        (:then_1
          (CallFunction|UpdateFOV)
          (Default|UpdateMoney (Variables|Default|GetGameInstance) DeltaSeconds)
          ;[0.15 0.15 0.15 0.5] HUD Update Money
          (if (Variables|Default|GetHUDOpen)
            (Default|UpdateHUD (Variables|Default|GetHUD) (Variables|/Game/LD57/Blueprints/BP_GameInstance.BP_GameInstance_C|GetMoney _gameinstance_2) (Variables|/Game/LD57/Blueprints/BP_GameInstance.BP_GameInstance_C|GetMoneyPerSecond _gameinstance_2) (Variables|/Game/LD57/Blueprints/BP_GameInstance.BP_GameInstance_C|GetCurrentLife _gameinstance_2) (Variables|/Game/LD57/Blueprints/BP_GameInstance.BP_GameInstance_C|GetRunTimer _gameinstance_2) (Variables|/Game/LD57/Blueprints/BP_GameInstance.BP_GameInstance_C|GetTimer _gameinstance_2))))
        (:then_2
          (bind (_clicklocation _valid _clickable) (CallFunction|GetClickLocation))
          (if (Variables|Default|GetHUDOpen)
            (Default|ShowCrosshair (Variables|Default|GetHUD) (and _valid _clickable))))
        (:then_3
          (if (Variables|Default|GetHUDOpen)
            (Default|ReduceTutoDuration (Variables|Default|GetHUD) DeltaSeconds)))
        (:then_4
          (if (Variables|/Game/LD57/Blueprints/BP_GameInstance.BP_GameInstance_C|GetRunTimer _gameinstance)
            (Variables|/Game/LD57/Blueprints/BP_GameInstance.BP_GameInstance_C|SetTimer _gameinstance (+ (Variables|/Game/LD57/Blueprints/BP_GameInstance.BP_GameInstance_C|GetTimer _gameinstance) DeltaSeconds))))))))

(event EventPossess
  (params (PossessedPawn :type Pawn%20Object%20Reference))
  (bind _asbp_player_character (Utilities|Casting|CastToBP_PlayerCharacter PossessedPawn))
  (bind _output_get (Variables|Default|SetPlayerCharacter _asbp_player_character))
  (Utilities|IsValid _output_get
    (:Is%20Valid
      (Variables|Default|SetInitialFOV (Variables|/Script/Engine.CameraComponent|GetFieldOfView (Variables|/Game/LD57/Blueprints/Player/BP_PlayerCharacter.BP_PlayerCharacter_C|GetTPSCamera _output_get)))
      (Class|PlayerController|SetAudioListenerOverride (Variables|/Script/Engine.Character|GetMesh _output_get) "0, 0, 0" "0, 0, 0"))))

(event EventUnPossess
  (params (UnpossessedPawn :type Pawn%20Object%20Reference))
  (Variables|Default|SetPlayerCharacter 0)
  (Class|PlayerController|SetAudioListenerOverride 0 "0, 0, 0" "0, 0, 0"))

(event Input|KeyboardEvents|DebugKeyDollar
  (params (Key :type Key%20Structure :default "None") (ActionValue :type Input%20Action%20Value%20Structure))
  (bind _gameinstance (Variables|Default|GetGameInstance))
  (:Pressed
    (Variables|/Game/LD57/Blueprints/BP_GameInstance.BP_GameInstance_C|SetMoney _gameinstance 1e+16)
    (Variables|/Game/LD57/Blueprints/BP_GameInstance.BP_GameInstance_C|SetRunTimer _gameinstance true)
    (Default|BuyUpgrade _gameinstance "NewEnumerator14")))

(event Input|KeyboardEvents|Dollar
  (params (Key :type Key%20Structure :default "None"))
  (:Pressed
    (Audio|PlaySound2D "/Game/LD57/Sound/Mais_t’es_pas_net_Baptiste_Cue.Mais_t’es_pas_net_Baptiste_Cue" 1.0 1.0 0.0 0 0)))

(fn ConstructionScript)

(fn UpdateFOV
  (bind _playercharacter (Variables|Default|GetPlayerCharacter))
  (bind _playercharacter_2 (Variables|Default|GetPlayerCharacter))
  (bind _initialfov (Variables|Default|GetInitialFOV))
  (bind _charactermovement (Variables|/Script/Engine.Character|GetCharacterMovement _playercharacter))
  (bind _tpscamera (Variables|/Game/LD57/Blueprints/Player/BP_PlayerCharacter.BP_PlayerCharacter_C|GetTPSCamera _playercharacter_2))
  (bind _returnvalue (Pawn|Components|CharacterMovement|GetLastUpdateVelocity _charactermovement))
  (Utilities|IsValid _playercharacter
    (:Is%20Valid
      (if (Variables|/Game/LD57/Blueprints/BP_GameInstance.BP_GameInstance_C|GetEnableFov (Variables|Default|GetGameInstance))
        (Camera|SetFieldOfView _tpscamera (Math|Float|SelectFloat (+ (* (- (Variables|Default|GetMaxFOV) _initialfov) (Math|Float|Clamp(Float) (/ (.z _returnvalue) (Default|GetVelocityMax (Variables|Default|GetGameInstance))))) _initialfov) _initialfov (< (.z _returnvalue) 0.0)))
        (else
          (Camera|SetFieldOfView _tpscamera (Variables|Default|GetInitialFOV)))))))

(fn GetClickLocation
  (bind _playercharacter (Variables|Default|GetPlayerCharacter))
  (bind _tpscamera (Variables|/Game/LD57/Blueprints/Player/BP_PlayerCharacter.BP_PlayerCharacter_C|GetTPSCamera _playercharacter))
  (bind _returnvalue (Transformation|GetWorldLocation _tpscamera))
  (Utilities|IsValid _playercharacter
    (:Is%20Valid
      (bind (_outhit _returnvalue_2) (Collision|LineTraceByChannel _returnvalue (+ _returnvalue (* (Math|Vector|GetForwardVector _tpscamera) (Variables|Default|GetClickLength))) "TraceTypeQuery1" false 0 "None"))
      (if _returnvalue_2
        (return (.impactpoint _outhit) true (Utilities|DoesObjectImplementInterface (.hitactor _outhit) "/Game/LD57/Blueprints/BPI_Clickable.BPI_Clickable_C") (.hitactor _outhit))
        (else
          (return "0, 0, 0" false false 0))))
    (:Is%20Not%20Valid
      (return "0, 0, 0" false false 0))))

(fn ToggleSkin
  (bind _output_get (Variables|Default|SetSkinOpen (not (Variables|Default|GetSkinOpen))))
  (if _output_get
    (Widget|RemovefromParent (Variables|Default|GetHUD))
    (UserInterface|Viewport|AddtoViewport (Variables|Default|GetSkinScreen) 0)
    (Variables|Default|SetbShowMouseCursor true)
    (else
      (Widget|RemovefromParent (Variables|Default|GetSkinScreen))
      (UserInterface|Viewport|AddtoViewport (Variables|Default|GetHUD) 0)
      (Variables|Default|SetbShowMouseCursor false)))
  (bind _newcamera (Default|SwitchCamera (Variables|Default|GetPlayerCharacter) (not _output_get)))
  (Utilities|IsValid _newcamera
    (:Is%20Valid
      (Game|Player|SetViewTargetwithBlend (Components|GetOwner _newcamera) 2.0 "VTBlend_EaseInOut" 1.0 false))))

(fn ToggleSettings
  (bind _output_get (Variables|Default|SetSettingsOpen (not (Variables|Default|GetSettingsOpen))))
  (if _output_get
    (Widget|RemovefromParent (Variables|Default|GetHUD))
    (UserInterface|Viewport|AddtoViewport (Variables|Default|GetSettingsScreen) 0)
    (Variables|Default|SetbShowMouseCursor true)
    (else
      (Widget|RemovefromParent (Variables|Default|GetSettingsScreen))
      (UserInterface|Viewport|AddtoViewport (Variables|Default|GetHUD) 0)
      (Variables|Default|SetbShowMouseCursor false))))