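; BP_Generator is a world actor for one purchasable income generator tier, identified by Level, with a dancing NPC and its own looping or ambient sound.
; Every tick it reads count, CPS, price and affordability from BP_GameInstance and pushes them to a WBP_GeneratorTextes widget.
; OnClick tries to buy the generator through the game instance, plays an upgrade or blocked sound, and returns whether it succeeded.
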(event EventBeginPlay
  (bind _asbp_game_instance (Utilities|Casting|CastToBP_GameInstance (Game|GetGameInstance)))
  (Variables|Default|SetGameInstance _asbp_game_instance)
  (bind _aswbp_generator_textes (Utilities|Casting|CastToWBP_GeneratorTextes (UserInterface|GetWidget (Variables|Default|GetTextes))))
  (Variables|Default|SetTextesWidget _aswbp_generator_textes)
  (CallFunction|Update)
  (Components|Animation|PlayAnimation (Variables|Default|GetPNJ) (Variables|Default|GetDance) true)
  (Audio|Components|Audio|SetSound (Variables|Default|GetAudio) (Variables|Default|GetSound)))

(event EventTick
  (params (DeltaSeconds :type Float%20%28single-precision%29))
  (CallFunction|Update))

(fn ConstructionScript)

(fn Update
  (bind _level (Variables|Default|GetLevel))
  (bind _gameinstance (Variables|Default|GetGameInstance))
  (bind _generator (Default|GetGenerator _gameinstance _level))
  (bind _price (Default|GetGeneratorPrice _gameinstance _level))
  (Default|UpdateTextes (Variables|Default|GetTextesWidget) (.currentcount _generator) (* (.cps _generator) (.currentcount _generator)) (Math|Conversions|ToFloat(Integer) _price) (>= (Variables|/Game/LD57/Blueprints/BP_GameInstance.BP_GameInstance_C|GetMoney _gameinstance) _price)))

(fn OnClick
  (params (Location :type Vector :default "0, 0, 0"))
  (bind _bought (Default|BuyGenerator (Variables|Default|GetGameInstance) (Variables|Default|GetLevel)))
  (Audio|PlaySoundatLocation (select _bought "/Game/LD57/Sound/Upgrade/SC_Upgrade.SC_Upgrade" "/Game/LD57/Sound/Blocked/SC_Blocked.SC_Blocked") Location "0, 0, 0" 1.0 1.0 0.0 0 0 0 0)
  (return _bought))