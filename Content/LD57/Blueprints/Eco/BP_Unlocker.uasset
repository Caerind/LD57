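; BP_Unlocker is a clickable shop object that sells a single upgrade, set by its Upgrade variable.
; It reads the upgrade's name, price and unlocked state from BP_GameInstance and refreshes its WBP_UnlockerTextes widget every tick, including whether the player can afford it.
; OnClick delegates the purchase to the game instance, plays a success or blocked sound at the given location, and returns the result.
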(event EventTick
  (params (DeltaSeconds :type Float%20%28single-precision%29))
  (bind _upgrade (Variables|Default|GetUpgrade))
  (bind _gameinstance (Variables|Default|GetGameInstance))
  (bind _upgrade_2 (Default|GetUpgrade _gameinstance _upgrade))
  (Default|UpdateTextes (Variables|Default|GetTextesWidget) (.unlocked _upgrade_2) (.name _upgrade_2) (Math|Conversions|ToInteger(Byte) (.price _upgrade_2)) (>= (Variables|/Game/LD57/Blueprints/BP_GameInstance.BP_GameInstance_C|GetMoney _gameinstance) (.price _upgrade_2))))

(event EventBeginPlay
  (bind _asbp_game_instance (Utilities|Casting|CastToBP_GameInstance (Game|GetGameInstance)))
  (Variables|Default|SetGameInstance _asbp_game_instance)
  (bind _aswbp_unlocker_textes (Utilities|Casting|CastToWBP_UnlockerTextes (UserInterface|GetWidget (Variables|Default|GetWidget))))
  (bind _output_get (Variables|Default|SetTextesWidget _aswbp_unlocker_textes))
  (Default|UpdateTextes _output_get (.unlocked (Default|GetUpgrade (Variables|Default|GetGameInstance) (Variables|Default|GetUpgrade))) (.name (Default|GetUpgrade (Variables|Default|GetGameInstance) (Variables|Default|GetUpgrade))) (Math|Conversions|ToInteger(Byte) (.price (Default|GetUpgrade (Variables|Default|GetGameInstance) (Variables|Default|GetUpgrade)))) false))

(fn ConstructionScript)

(fn OnClick
  (params (Location :type Vector :default "0, 0, 0"))
  (bind _bought (Default|BuyUpgrade (Variables|Default|GetGameInstance) (Variables|Default|GetUpgrade)))
  (Audio|PlaySoundatLocation (select _bought "/Game/LD57/Sound/Upgrade/SC_Upgrade.SC_Upgrade" "/Game/LD57/Sound/Blocked/SC_Blocked.SC_Blocked") Location "0, 0, 0" 1.0 1.0 0.0 0 0 0 0)
  (return _bought))