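; BP_HardcodeToggler is a clickable text label that switches the game's hardcore mode on and off.
; On BeginPlay it caches BP_GameInstance, which holds the HardcodeEnabled flag, and refreshes its TextRender.
; OnClick calls ToggleHardcoreMode on the game instance, refreshes the label, plays SC_Blocked at the click location and returns true.
; Update derives both the text color and the On/Off wording from that flag.
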(event EventBeginPlay
  (bind _asbp_game_instance (Utilities|Casting|CastToBP_GameInstance (Game|GetGameInstance)))
  (Variables|Default|SetGameInstance _asbp_game_instance)
  (CallFunction|Update))

(fn ConstructionScript)

(fn Update
  (bind _textrender (Variables|Default|GetTextRender))
  (bind _gameinstance (Variables|Default|GetGameInstance))
  (bind _hardcodeenabled (Variables|/Game/LD57/Blueprints/BP_GameInstance.BP_GameInstance_C|GetHardcodeEnabled _gameinstance))
  (Rendering|Components|TextRender|SetTextRenderColor _textrender (select _hardcodeenabled (LocalVariables|GetTrueColor) (LocalVariables|GetFalseColor)))
  (Rendering|Components|TextRender|SetText _textrender (Utilities|Text|ToText(String) (Utilities|String|SelectString "Hardcore: On" "Hardcore: Off" _hardcodeenabled))))

(fn OnClick
  (params (Location :type Vector :default "0, 0, 0"))
  (Default|ToggleHardcoreMode (Variables|Default|GetGameInstance))
  (CallFunction|Update)
  (Audio|PlaySoundatLocation "/Game/LD57/Sound/Blocked/SC_Blocked.SC_Blocked" Location "0, 0, 0" 1.0 1.0 0.0 0 0 0 0)
  (return true))