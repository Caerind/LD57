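; Trigger actor that litters an area with corpses reflecting the lives the player has wasted so far.
; The first player overlap of CollisionBox reads TotalLifeWasted from BP_GameInstance and loops a spawn on that count, guarded by a Done flag.
; Each BP_Cadavre appears at a random point inside SpawnBox with a random rotation, adjusted for collision but always spawned.
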(event OnComponentBeginOverlap(CollisionBox)
  (params (OverlappedComponent :type Primitive%20Component%20Object%20Reference) (OtherActor :type Actor%20Object%20Reference) (OtherComp :type Primitive%20Component%20Object%20Reference) (OtherBodyIndex :type Integer) (bFromSweep :type Boolean) (SweepResult :type Hit%20Result%20Structure%20%28by%20ref%29))
  (Utilities|Casting|CastToBP_PlayerCharacter OtherActor)
  (if (not (Variables|Default|GetDone))
    (Variables|Default|SetDone true)
    (bind _asbp_game_instance (Utilities|Casting|CastToBP_GameInstance (Game|GetGameInstance)))
    (for _index (range 0 (Variables|/Game/LD57/Blueprints/BP_GameInstance.BP_GameInstance_C|GetTotalLifeWasted _asbp_game_instance))
      (CallFunction|SpawnCadavre))))

(event Custom|SpawnCadavre
  (bind _spawnbox (Variables|Default|GetSpawnBox))
  ;[0.15 0.15 0.15 0.5] Spawn un cadavre dans la box
  (Game|SpawnActorfromClass "/Game/LD57/Blueprints/LD/BP_Cadavre.BP_Cadavre_C" (Math|Transform|MakeTransform (Math|Random|RandomPointinBoundingBox (Transformation|GetWorldLocation _spawnbox) (Components|Box|GetScaledBoxExtent _spawnbox)) (Math|Random|RandomRotator false) "1.000000,1.000000,1.000000") "AdjustIfPossibleButAlwaysSpawn" "MultiplyWithRoot" 0 0))

(fn ConstructionScript)