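; BP_TimerStop is a finish-line trigger that stops the run timer and submits the player's time to an online leaderboard.
; When BP_PlayerCharacter overlaps the box, it clears RunTimer on BP_GameInstance, so it fires only while a run is active.
; With a username set, it converts the timer to a score and sends it by HTTP GET to the normal or hardcore dreamlo board.
; Both leaderboard displays refresh whether the request succeeds or fails.
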(event OnComponentBeginOverlap(Box)
  (params (OverlappedComponent :type Primitive%20Component%20Object%20Reference) (OtherActor :type Actor%20Object%20Reference) (OtherComp :type Primitive%20Component%20Object%20Reference) (OtherBodyIndex :type Integer) (bFromSweep :type Boolean) (SweepResult :type Hit%20Result%20Structure%20%28by%20ref%29))
  (Utilities|Casting|CastToBP_PlayerCharacter OtherActor)
  (bind _asbp_game_instance (Utilities|Casting|CastToBP_GameInstance (Game|GetGameInstance)))
  (if (Variables|/Game/LD57/Blueprints/BP_GameInstance.BP_GameInstance_C|GetRunTimer _asbp_game_instance)
    (Variables|/Game/LD57/Blueprints/BP_GameInstance.BP_GameInstance_C|SetRunTimer _asbp_game_instance false)
    (if (not (Utilities|Array|IsEmpty (Variables|/Game/LD57/Blueprints/BP_GameInstance.BP_GameInstance_C|GetUsername _asbp_game_instance)))
      (if (Variables|/Game/LD57/Blueprints/BP_GameInstance.BP_GameInstance_C|GetHardcodeEnabled _asbp_game_instance)
        (bind _result_body (|HttpRequest (Utilities|String|Append "http://dreamlo.com/lb/" (Variables|Default|GetHardcoreWriteToken) "/add/" (Variables|/Game/LD57/Blueprints/BP_GameInstance.BP_GameInstance_C|GetUsername _asbp_game_instance) "/" (Utilities|String|ToString(Integer) (Default|TimertoScore (Variables|Default|GetNormalLeaderboard) (Variables|/Game/LD57/Blueprints/BP_GameInstance.BP_GameInstance_C|GetTimer _asbp_game_instance)))) "Get")
          (:On%20Success
            _)
          (:On%20Error
            _))
        (else
          (bind _result_body_2 (|HttpRequest (Utilities|String|Append "http://dreamlo.com/lb/" (Variables|Default|GetNormalWriteToken) "/add/" (Variables|/Game/LD57/Blueprints/BP_GameInstance.BP_GameInstance_C|GetUsername _asbp_game_instance) "/" (Utilities|String|ToString(Integer) (Default|TimertoScore (Variables|Default|GetNormalLeaderboard) (Variables|/Game/LD57/Blueprints/BP_GameInstance.BP_GameInstance_C|GetTimer _asbp_game_instance)))) "Get")
            (:On%20Success
              _)
            (:On%20Error
              _))))
      (Default|UpdateLeaderboard (Variables|Default|GetNormalLeaderboard))
      (Default|UpdateLeaderboard (Variables|Default|GetHardcoreLeaderboard)))))

(fn ConstructionScript)