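; BP_PortalRestart is a portal that restarts the run when the player character overlaps its Plane component.
; On overlap it destroys every BP_Cadavre actor, then teleports player 0's character to the location and rotation of the PlayerStart found in the level.
; It also resets the GameInstance timer to zero and restores current life to the max life count, all without reloading the level.
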(event OnComponentBeginOverlap(Plane)
  (params (OverlappedComponent :type Primitive%20Component%20Object%20Reference) (OtherActor :type Actor%20Object%20Reference) (OtherComp :type Primitive%20Component%20Object%20Reference) (OtherBodyIndex :type Integer) (bFromSweep :type Boolean) (SweepResult :type Hit%20Result%20Structure%20%28by%20ref%29))
  (bind _asbp_player_character (Utilities|Casting|CastToBP_PlayerCharacter OtherActor))
  (Utilities|FlowControl|Sequence
    (:then_0
      (bind _outactors (Actor|GetAllActorsOfClass "/Game/LD57/Blueprints/LD/BP_Cadavre.BP_Cadavre_C"))
      (for _array_element _outactors
        (Actor|DestroyActor _array_element)))
    (:then_1
      (bind _returnvalue (Actor|GetActorOfClass "/Script/Engine.PlayerStart"))
      (Transformation|SetActorLocationAndRotation (Game|GetPlayerCharacter 0) (Transformation|GetActorLocation _returnvalue) (Transformation|GetActorRotation _returnvalue) false true))
    (:then_2
      (Variables|/Game/LD57/Blueprints/BP_GameInstance.BP_GameInstance_C|SetTimer (Variables|/Game/LD57/Blueprints/Player/BP_PlayerCharacter.BP_PlayerCharacter_C|GetGameInstance _asbp_player_character) 0.0))
    (:then_3
      (Variables|/Game/LD57/Blueprints/BP_GameInstance.BP_GameInstance_C|SetCurrentLife (Variables|/Game/LD57/Blueprints/Player/BP_PlayerCharacter.BP_PlayerCharacter_C|GetGameInstance _asbp_player_character) (Default|GetMaxLifeCount (Variables|/Game/LD57/Blueprints/Player/BP_PlayerCharacter.BP_PlayerCharacter_C|GetGameInstance _asbp_player_character))))))

(fn ConstructionScript)