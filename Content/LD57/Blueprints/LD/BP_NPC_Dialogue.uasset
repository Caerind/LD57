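; BP_NPC_Dialogue is an NPC Blueprint that shows dialogue as in-world text.
; On BeginPlay it applies its SkeletalMesh variable to the mesh, then casts the DialogueWidget component's widget to WBP_InWorldText and passes it the Dialogue value.
; Both mesh and text come from variables, and the construction script only calls its parent.
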(event EventBeginPlay
  (|CallParentFunction)
  (Components|SkeletalMesh|SetSkeletalMeshAsset (Variables|Character|GetMesh) (Variables|Default|GetSkeletalMesh))
  (bind _aswbp_in_world_text (Utilities|Casting|CastToWBP_InWorldText (UserInterface|GetWidget (Variables|Default|GetDialogueWidget))))
  (Default|SetString _aswbp_in_world_text (Variables|Default|GetDialogue)))

(fn ConstructionScript
  (|CallParentFunction))