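; BP_TimerStart is a trigger volume that marks the start zone for the run timer.
; It caches BP_GameInstance on BeginPlay.
; While the player character overlaps its Box, it stops the timer.
; When the player leaves, it resets the timer to zero and starts it running through flags on the game instance.
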(event OnComponentEndOverlap(Box)
  (params (OverlappedComponent :type Primitive%20Component%20Object%20Reference) (OtherActor :type Actor%20Object%20Reference) (OtherComp :type Primitive%20Component%20Object%20Reference) (OtherBodyIndex :type Integer))
  (bind _gameinstance (Variables|Default|GetGameInstance))
  (Utilities|Casting|CastToBP_PlayerCharacter OtherActor)
  (Variables|/Game/LD57/Blueprints/BP_GameInstance.BP_GameInstance_C|SetTimer _gameinstance 0.0)
  (Variables|/Game/LD57/Blueprints/BP_GameInstance.BP_GameInstance_C|SetRunTimer _gameinstance true))

(event OnComponentBeginOverlap(Box)
  (params (OverlappedComponent :type Primitive%20Component%20Object%20Reference) (OtherActor :type Actor%20Object%20Reference) (OtherComp :type Primitive%20Component%20Object%20Reference) (OtherBodyIndex :type Integer) (bFromSweep :type Boolean) (SweepResult :type Hit%20Result%20Structure%20%28by%20ref%29))
  (Utilities|Casting|CastToBP_PlayerCharacter OtherActor)
  (Variables|/Game/LD57/Blueprints/BP_GameInstance.BP_GameInstance_C|SetRunTimer (Variables|Default|GetGameInstance) false))

(event EventBeginPlay
  (bind _asbp_game_instance (Utilities|Casting|CastToBP_GameInstance (Game|GetGameInstance)))
  (Variables|Default|SetGameInstance _asbp_game_instance))

(fn ConstructionScript)